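; Game mode Blueprint that serves as a test bed for dynamic delegates.
; On BeginPlay it passes custom events as delegate arguments to TestFuncDynamicStandardDelegate and TestFuncDynamicMulticastDelegate.
; The two events given to the multicast test print differently colored messages, while the standard test's event is empty.
; Bindings to MyDyMulticastDelegate and its one-parameter variant exist but are unconnected, so they never run.
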(event Custom|CustomEvent_0)

(event Custom|CustomEvent_1
  (params (Str :type String)))

(event Custom|CustomEvent_2)

(event Custom|CustomEvent_3
  (Development|PrintString "My dynamic standard delegate 1" true true "(R=0.000000,G=0.140520,B=1.000000,A=1.000000)" 123.0))

(event Custom|CustomEvent_4
  (Development|PrintString "My dynamic standard delegate 2" true true "(R=1.000000,G=0.940505,B=0.000000,A=1.000000)" 123.0))

(event EventBeginPlay
  (Class|MyGameMode|TestFuncDynamicStandardDelegate (delegate Custom|CustomEvent_2))
  (Class|MyGameMode|TestFuncDynamicMulticastDelegate (delegate Custom|CustomEvent_3) (delegate Custom|CustomEvent_4)))

(event EventTick
  (params (DeltaSeconds :type Float%20%28single-precision%29)))

(fn ConstructionScript)